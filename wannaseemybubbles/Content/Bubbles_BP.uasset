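; Bubbles_BP is a player-controlled Blueprint that runs timed shifts with a score quota.
; It adds an Enhanced Input mapping context, handles look with inverted pitch, and line-traces from the camera on interact.
; Hitting a "Monitor"-tagged actor starts the next shift, setting time and quota by shift number.
; A one-second Delay loop counts down, then prints PASS or DEAD by comparing Score, which is not changed here, to Quota.
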(event `Next shift`
  ;[1 0 0.05 1 35] New shift
  (set `self.shift` (+ (`self.shift`) 1))
  (`self.Set timer`)
  (`self.Set quota`)
  (set `self.ispaused` false)
  (`self.Timer`))

(event `self.ReceiveBeginPlay`
  ;[1 0 0.05 1 35] BeginPlay
  (bind _asplayer_controller (cast `PlayerController` (`self.GetController`)))
  (`EnhancedInputSubsystemInterface.AddMappingContext` (pcsubsystem `EnhancedInputLocalPlayerSubsystem` _asplayer_controller) "/Game/IMC.IMC" 0 (struct)))

(event `Set timer`
  ;[0 0.1608 1 1 25] Set timer
  (if (== (`self.shift`) 1)
    (set `self.remainingtime` 60)
    (else
      (set `self.remainingtime` 30))))

(event `EnhancedInput|/Game/IA_Look`
  (params (ActionValue :type "Vector2D Structure") (ElapsedSeconds :type "Float (double-precision)") (TriggeredSeconds :type "Float (double-precision)") (InputAction :type "InputAction Object Reference" :default "/Game/IA_Look.IA_Look"))
  ;[1 0 0.05 1 25] Look
  (:`Triggered`
    (`self.AddControllerYawInput` ActionValue_X)
    (`self.AddControllerPitchInput` (- ActionValue_Y (* ActionValue_Y 2.0)))))

(event `Set quota`
  ;[0 0.1608 1 1 25] Set quota
  (if (<= (`self.shift`) 2)
    (set `self.quota` 4)
    (else
      (set `self.quota` 8))))

(event `Timer`
  ;[0 0.1608 1 1 25] Timer
  (while (`KismetMathLibrary.BooleanNOR` (`self.ispaused`) (<= (`self.remainingtime`) 0)) :!label _label
    (`KismetSystemLibrary.Delay` 1.0)
    (set `self.remainingtime` (- (`self.remainingtime`) 1))
    (goto _label))
  (if (>= (`self.score`) (`self.quota`))
    (`KismetSystemLibrary.PrintString` "PASS")
    (else
      (`KismetSystemLibrary.PrintString` "DEAD"))))

(event `EnhancedInput|/Game/IA_Interact`
  (params (ActionValue :type Boolean) (ElapsedSeconds :type "Float (double-precision)") (TriggeredSeconds :type "Float (double-precision)") (InputAction :type "InputAction Object Reference" :default "/Game/IA_Interact.IA_Interact"))
  (bind _camera (`self.Camera`))
  (bind _returnvalue (`SceneComponent.K2_GetComponentLocation` _camera))
  ;[1 0.1304 0 1 25] Interact
  (:`Triggered`
    (bind (_outhit _returnvalue_2) (`KismetSystemLibrary.LineTraceSingle` :`Start` _returnvalue :`End` (+ _returnvalue (* (`KismetMathLibrary.GetForwardVector` (`SceneComponent.K2_GetComponentRotation` _camera)) 1000.0)) :`TraceChannel` "TraceTypeQuery1" :`DrawDebugType` "ForDuration" :`DrawTime` 1.0))
    (if _returnvalue_2
      (if (`self.ActorHasTag` (`.HitActor` (`GameplayStatics.BreakHitResult` _outhit)) "Monitor")
        (`self.Next shift`)))))

(fn `UserConstructionScript`)